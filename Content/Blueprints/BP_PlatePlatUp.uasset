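; Pressure plate that moves a linked door actor (BPDoor2) while an object tagged "Object" rests on it.
; Box overlaps toggle DoorOpen and switch the plate and optional Line mesh between green and red materials.
; Tick plays or reverses a timeline that offsets the door from its starting location, also opening if optional BPLPlate is open.
; Tick also sets Occupied when multiple Characters overlap the box, which blocks overlap changes.
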(event OnComponentBeginOverlap(Box)
  (params (OverlappedComponent :type Primitive%20Component%20Object%20Reference) (OtherActor :type Actor%20Object%20Reference) (OtherComp :type Primitive%20Component%20Object%20Reference) (OtherBodyIndex :type Integer) (bFromSweep :type Boolean) (SweepResult :type Hit%20Result%20Structure%20%28by%20ref%29))
  (if (not (Variables|Default|GetOccupied))
    (if (Actor|ActorHasTag OtherActor "Object")
      (Variables|Default|SetDoor%20Open true)
      (Rendering|Material|SetMaterial (Variables|Default|GetPlane) 0 "/Game/Mat-Tex/M_PlateGreen.M_PlateGreen")
      (bind _line (Variables|Default|GetLine)
        (:then
          (for _index (range 0 (Utilities|Array|Length (Rendering|Material|GetMaterials (Variables|/Game/Blueprints/BP_Line.BP_Line_C|GetStaticMesh _line))))
            (Rendering|Material|SetMaterial (Variables|/Game/Blueprints/BP_Line.BP_Line_C|GetStaticMesh _line) _index "/Game/Mat-Tex/M_PlateGreen.M_PlateGreen")))
        (:else)))))

(event OnComponentEndOverlap(Box)
  (params (OverlappedComponent :type Primitive%20Component%20Object%20Reference) (OtherActor :type Actor%20Object%20Reference) (OtherComp :type Primitive%20Component%20Object%20Reference) (OtherBodyIndex :type Integer))
  (if (not (Variables|Default|GetOccupied))
    (if (Actor|ActorHasTag OtherActor "Object")
      (Variables|Default|SetDoor%20Open false)
      (Rendering|Material|SetMaterial (Variables|Default|GetPlane) 0 "/Game/Mat-Tex/M_PlateRed.M_PlateRed")
      (bind _line (Variables|Default|GetLine)
        (:then
          (for _index (range 0 (Utilities|Array|Length (Rendering|Material|GetMaterials (Variables|/Game/Blueprints/BP_Line.BP_Line_C|GetStaticMesh _line))))
            (Rendering|Material|SetMaterial (Variables|/Game/Blueprints/BP_Line.BP_Line_C|GetStaticMesh _line) _index "/Game/Mat-Tex/M_PlateRed.M_PlateRed")))
        (:else)))))

(event EventBeginPlay
  (Variables|Default|SetDoorLocation (Transformation|GetActorLocation (Variables|Default|GetBP_Door2))))

(event EventTick
  (params (DeltaSeconds :type Float%20%28single-precision%29))
  (Utilities|FlowControl|Sequence
    (:then_0
      (bind _bp_lplate (Variables|Default|GetBP_LPlate)
        (:then
          (if (or (Variables|Default|GetDoor%20Open) (Variables|/Game/Blueprints/BP_Plate.BP_Plate_C|GetDoor%20Open _bp_lplate))
            (bind _slide_down (Timeline|Door%20Down Play)
              (:Update
                (Transformation|SetActorRelativeLocation (Variables|Default|GetBP_Door2) (+ _slide_down (Variables|Default|GetDoorLocation)))))
            (else
              (Timeline|Door%20Down Reverse))))
        (:else
          (if (Variables|Default|GetDoor%20Open)
            (Timeline|Door%20Down Play)
            (else
              (Timeline|Door%20Down Reverse))))))
    (:then_1
      (if (> (Utilities|Array|Length (Collision|GetOverlappingActors (Variables|Default|GetBox) "/Script/Engine.Character" :!class /Script/Engine.PrimitiveComponent)) 1)
        (Variables|Default|SetOccupied true)
        (else
          (Variables|Default|SetOccupied false))))))

(fn ConstructionScript)