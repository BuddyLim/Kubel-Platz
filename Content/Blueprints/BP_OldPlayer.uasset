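; BP_OldPlayer is a player pawn that moves, drops BP_CubeClone copies and collects BP_Bananana pickups.
; Axis input accumulates movement vectors that Tick consumes as a swept local offset.
; SpawnCube places clones at the pawn's transform on a short cooldown, stores them and creates a dynamic material on the pawn's mesh.
; Overlapped bananas are destroyed and counted, driving that material's ColorAlpha.
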(event OnComponentBeginOverlap(StaticMesh)
  (params (OverlappedComponent :type Primitive%20Component%20Object%20Reference) (OtherActor :type Actor%20Object%20Reference) (OtherComp :type Primitive%20Component%20Object%20Reference) (OtherBodyIndex :type Integer) (bFromSweep :type Boolean) (SweepResult :type Hit%20Result%20Structure%20%28by%20ref%29))
  (bind _asbp_bananana (Utilities|Casting|CastToBP_Bananana OtherActor))
  (Actor|DestroyActor _asbp_bananana)
  (bind _result (Math|Float|IncrementFloat (Variables|Default|GetBananaCounter))
    (:%20%20
      (Rendering|Material|SetScalarParameterValue (Variables|Default|GetCubeMaterial) "ColorAlpha" (Math|Float|Clamp(Float) (/ _result 6.0)) :!class /Script/Engine.MaterialInstanceDynamic))))

(event EventTick
  (params (DeltaSeconds :type Float%20%28single-precision%29))
  (Utilities|FlowControl|Sequence
    (:then_0
      (bind _returnvalue (Class|Pawn|ConsumeMovementInputVector))
      (Transformation|AddActorLocalOffset (* _returnvalue DeltaSeconds) true false))))

(event Input|AxisEvents|InputAxisForwardMovement
  (params (AxisValue :type Float%20%28single-precision%29))
  (Pawn|Input|AddMovementInput (Transformation|GetActorForwardVector) (* AxisValue (Variables|Default|GetMaxSpeed)) true))

(event Input|AxisEvents|InputAxisSideMovement
  (params (AxisValue :type Float%20%28single-precision%29))
  (Pawn|Input|AddMovementInput (Transformation|GetActorRightVector) (* AxisValue (Variables|Default|GetMaxSpeed)) true))

(event Input|AxisEvents|InputAxisSpawnCube
  (params (AxisValue :type Float%20%28single-precision%29))
  (if (and (== AxisValue 1.0) (Variables|Default|GetCanSpawn))
    (bind _returnvalue (Game|SpawnActorfromClass "/Game/Blueprints/BP_CubeClone.BP_CubeClone_C" (Transformation|GetActorTransform) "Undefined" 0 0))
    (Utilities|FlowControl|Sequence
      (:then_1
        (Utilities|Array|Add (Variables|Default|GetBC_Array) _returnvalue)
        (bind _returnvalue_2 (Rendering|Material|CreateDynamicMaterialInstance (Variables|Default|GetStaticMesh) 0 "/Game/Mat-Tex/PlayerColor.PlayerColor" "None" :!class /Script/Engine.PrimitiveComponent))
        (Variables|Default|SetCubeMaterial _returnvalue_2)
        (Variables|Default|SetCanSpawn false)
        (Utilities|FlowControl|Delay 0.2)
        (Variables|Default|SetCanSpawn true)))))

(fn ConstructionScript)