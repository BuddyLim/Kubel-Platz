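; BP_SeeSaw is a seesaw that launches a character standing on its right side when a push block hits the left side.
; A BP_PushBlock overlapping Left sets Launch true for 0.1 seconds.
; Tick casts an overlap event's OtherActor to BP_Player or BP_Platz and, while Launch is set and that character overlaps Right, applies a fixed upward and +Y LaunchCharacter velocity.
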(event OnComponentBeginOverlap(Left)
  (params (OverlappedComponent :type Primitive%20Component%20Object%20Reference) (OtherActor :type Actor%20Object%20Reference) (OtherComp :type Primitive%20Component%20Object%20Reference) (OtherBodyIndex :type Integer) (bFromSweep :type Boolean) (SweepResult :type Hit%20Result%20Structure%20%28by%20ref%29))
  (Utilities|Casting|CastToBP_PushBlock OtherActor)
  (Variables|Default|SetLaunch true)
  (Utilities|FlowControl|Delay 0.1)
  (Variables|Default|SetLaunch false))

(event OnComponentBeginOverlap(Right)
  (params (OverlappedComponent :type Primitive%20Component%20Object%20Reference) (OtherActor :type Actor%20Object%20Reference) (OtherComp :type Primitive%20Component%20Object%20Reference) (OtherBodyIndex :type Integer) (bFromSweep :type Boolean) (SweepResult :type Hit%20Result%20Structure%20%28by%20ref%29)))

(event EventBeginPlay)

(event Collision|EventActorBeginOverlap
  (params (OtherActor :type Actor%20Object%20Reference)))

(event EventTick
  (params (DeltaSeconds :type Float%20%28single-precision%29))
  (bind _asbp_player (Utilities|Casting|CastToBP_Player (stale OnComponentBeginOverlap(Right) OtherActor))
    (:then
      (if (and (Collision|IsOverlappingActor (Variables|Default|GetRight) _asbp_player :!class /Script/Engine.PrimitiveComponent) (Variables|Default|GetLaunch))
        (Character|LaunchCharacter _asbp_player "0,25.000000,50.000000" false false)))
    (:CastFailed
      (bind _asbp_platz (Utilities|Casting|CastToBP_Platz (stale OnComponentBeginOverlap(Right) OtherActor)))
      (if (and (Collision|IsOverlappingActor (Variables|Default|GetRight) _asbp_platz :!class /Script/Engine.PrimitiveComponent) (Variables|Default|GetLaunch))
        (Character|LaunchCharacter _asbp_platz "0,25.000000,50.000000" false false)))))

(fn ConstructionScript)