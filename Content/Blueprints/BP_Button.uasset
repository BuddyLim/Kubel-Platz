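; BP_Button is an overlap-triggered button that respawns a push block.
; When anything begins overlapping its Sphere, it destroys the block it last spawned and spawns a new BP_PushBlock at the referenced BPSpawner's transform.
; The Cylinder and, if valid, every material slot on the linked Line mesh turn green.
; A one-second Delay inside the Line material loop leads to both being set back to red, so the reset requires a valid Line.
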(event OnComponentBeginOverlap(Sphere)
  (params (OverlappedComponent :type Primitive%20Component%20Object%20Reference) (OtherActor :type Actor%20Object%20Reference) (OtherComp :type Primitive%20Component%20Object%20Reference) (OtherBodyIndex :type Integer) (bFromSweep :type Boolean) (SweepResult :type Hit%20Result%20Structure%20%28by%20ref%29))
  (bind _bp_pushblock (Variables|Default|GetBP_Pushblock)
    (:then
      (Actor|DestroyActor _bp_pushblock))
    (:else
      _))
  (bind _returnvalue (Game|SpawnActorfromClass "/Game/Blueprints/BP_PushBlock.BP_PushBlock_C" (Transformation|GetActorTransform (Variables|Default|GetBP_Spawner)) "Undefined" 0 0))
  (Variables|Default|SetBP_Pushblock _returnvalue)
  (Rendering|Material|SetMaterial (Variables|Default|GetCylinder) 0 "/Game/Mat-Tex/M_PlateGreen.M_PlateGreen")
  (bind _line (Variables|Default|GetLine)
    (:then
      (for _index (range 0 (Utilities|Array|Length (Rendering|Material|GetMaterials (Variables|/Game/Blueprints/BP_Line.BP_Line_C|GetStaticMesh _line))))
        (Rendering|Material|SetMaterial (Variables|/Game/Blueprints/BP_Line.BP_Line_C|GetStaticMesh _line) _index "/Game/Mat-Tex/M_PlateGreen.M_PlateGreen")
        (Utilities|FlowControl|Delay 1.0)
        (Rendering|Material|SetMaterial (Variables|Default|GetCylinder) 0 "/Game/Mat-Tex/M_PlateRed.M_PlateRed")
        (bind _line_2 (Variables|Default|GetLine)
          (:then
            (for _index_2 (range 0 (Utilities|Array|Length (Rendering|Material|GetMaterials (Variables|/Game/Blueprints/BP_Line.BP_Line_C|GetStaticMesh _line_2))))
              (Rendering|Material|SetMaterial (Variables|/Game/Blueprints/BP_Line.BP_Line_C|GetStaticMesh _line_2) _index_2 "/Game/Mat-Tex/M_PlateRed.M_PlateRed")))
          (:else))))
    (:else)))

(event EventBeginPlay)

(event Collision|EventActorBeginOverlap
  (params (OtherActor :type Actor%20Object%20Reference)))

(event EventTick
  (params (DeltaSeconds :type Float%20%28single-precision%29)))

(fn ConstructionScript)