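; BP_Platz is an AI character that hunts down BP_CubeClone pawns.
; BeginPlay caches the player's BP_Player, whose BCArray supplies the targets.
; When PawnSensing sees a clone, it moves to the array's first entry rather than the seen pawn, then destroys and removes that entry on success.
; The overlap handler only casts, and a velocity-based jump is disabled.
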(event OnSeePawn(PawnSensing)
  (params (Pawn :type Pawn%20Object%20Reference))
  (Utilities|Casting|CastToBP_CubeClone Pawn)
  (AI|AIMoveTo self "0, 0, 0" (Utilities|Array|Get(acopy) (Variables|/Game/Blueprints/BP_Player.BP_Player_C|GetBCArray (stale EventBeginPlay _asbp_player))) 5.0 true
    (:OnSuccess
      (Actor|DestroyActor (Utilities|Array|Get(acopy) (Variables|/Game/Blueprints/BP_Player.BP_Player_C|GetBCArray (stale EventBeginPlay _asbp_player))))
      (Utilities|Array|RemoveItem (Variables|/Game/Blueprints/BP_Player.BP_Player_C|GetBCArray (stale EventBeginPlay _asbp_player)) (Utilities|Array|Get(acopy) (Variables|/Game/Blueprints/BP_Player.BP_Player_C|GetBCArray (stale EventBeginPlay _asbp_player)))))))

(event EventBeginPlay
  (bind _asbp_player (Utilities|Casting|CastToBP_Player (Game|Player|GetPlayerPawn 0))))

(event Collision|EventActorBeginOverlap
  (params (OtherActor :type Actor%20Object%20Reference))
  (Utilities|Casting|CastToBP_CubeClone OtherActor))

(event EventTick
  (params (DeltaSeconds :type Float%20%28single-precision%29)))

(fn ConstructionScript)